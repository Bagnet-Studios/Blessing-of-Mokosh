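; BP_NPC is a talkable NPC that shows its conversation one line at a time.
; On BeginPlay it caches DT_Dialogue rows matching its NPCID.
; Each Interact advances the line, turns the NPC toward the player, disables player movement and fills W_Dialogue with the matching ConversationID and LineID row.
; Without exactly one match it closes the widget, resets and restores walking; leaving the Box also removes the widget.
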(event OnComponentEndOverlap(Box)
  (params (OverlappedComponent :type Primitive%20Component%20Object%20Reference) (OtherActor :type Actor%20Object%20Reference) (OtherComp :type Primitive%20Component%20Object%20Reference) (OtherBodyIndex :type Integer))
  (Utilities|IsValid (Variables|Default|GetDialogueWidgetRef)
    (:Is%20Valid
      (Utilities|Casting|CastToBP_PlayerCharacter OtherActor)
      (Widget|RemovefromParent (Variables|Default|GetDialogueWidgetRef))
      (Variables|Default|SetDialogueWidgetRef 0))))

(event EventBeginPlay
  (bind _outrownames (DataTable|GetDataTableRowNames "/Game/Dialogue/DT_Dialogue.DT_Dialogue"))
  (for _array_element _outrownames
    (bind _returnvalue (Utilities|GetDataTableRow "/Game/Dialogue/DT_Dialogue.DT_Dialogue" _array_element)
      (:then
        (if (== (.NPC_ID (Utilities|Struct|BreakDS_Dialogue _returnvalue)) (Variables|Default|GetNPC_ID))
          (Utilities|Array|Add (Variables|Default|GetMyDialogue) _array_element))))))

(event EventInteract
  (Math|Integer|IncrementInt (Variables|Default|GetLineCurrent)
    (:%20%20
      (CallFunction|DialogueCreate)
      (Transformation|SetActorRotation (Math|Rotator|MakeRotator 0.0 0.0 (.yaw (Math|Rotator|FindLookatRotation (Transformation|GetActorLocation) (Transformation|GetActorLocation (Game|GetPlayerCharacter 0))))))
      (if (not (== (Variables|Default|GetLineCurrent) 0))
        (bind _asbp_player_character (Utilities|Casting|CastToBP_PlayerCharacter (Game|GetPlayerCharacter 0)))
        (Pawn|Components|CharacterMovement|DisableMovement (Variables|/Script/Engine.Character|GetCharacterMovement _asbp_player_character))))))

(fn ConstructionScript)

(fn DialogueCreate
  (Utilities|IsValid (Variables|Default|GetDialogueWidgetRef)
    (:Is%20Valid
      (bind (_returned_line _returned_name) (CallFunction|DialogueGetLine))
      (Variables|/Game/Dialogue/W_Dialogue.W_Dialogue_C|SetDialogueText (Variables|Default|GetDialogueWidgetRef) _returned_line)
      (Variables|/Game/Dialogue/W_Dialogue.W_Dialogue_C|SetName (Variables|Default|GetDialogueWidgetRef) _returned_name))
    (:Is%20Not%20Valid
      (bind _returnvalue (UserInterface|CreateWidget "/Game/Dialogue/W_Dialogue.W_Dialogue_C" (Game|GetPlayerController 0)))
      (bind _output_get (Variables|Default|SetDialogueWidgetRef _returnvalue))
      (UserInterface|Viewport|AddtoViewport _output_get 0)
      (bind (_returned_line_2 _returned_name_2) (CallFunction|DialogueGetLine))
      (Variables|/Game/Dialogue/W_Dialogue.W_Dialogue_C|SetDialogueText (Variables|Default|GetDialogueWidgetRef) _returned_line_2)
      (Variables|/Game/Dialogue/W_Dialogue.W_Dialogue_C|SetName (Variables|Default|GetDialogueWidgetRef) _returned_name_2))))

(fn DialogueGetLine
  (for _array_element (Variables|Default|GetMyDialogue)
    (bind _returnvalue (Utilities|GetDataTableRow "/Game/Dialogue/DT_Dialogue.DT_Dialogue" _array_element)
      (:then
        (if (and (== (.Conversation_ID (Utilities|Struct|BreakDS_Dialogue _returnvalue)) (Variables|Default|GetConversation_ID)) (== (.Line_ID (Utilities|Struct|BreakDS_Dialogue _returnvalue)) (Variables|Default|GetLineCurrent)))
          (Utilities|Array|Add (LocalVariables|GetReturnedLines) (.Dialogue (Utilities|Struct|BreakDS_Dialogue _returnvalue)))
          (Utilities|Array|Add (LocalVariables|GetReturnedName) (.Name (Utilities|Struct|BreakDS_Dialogue _returnvalue)))))))
  (if (== (Utilities|Array|Length (LocalVariables|GetReturnedLines)) 1)
    (return (Utilities|Array|Get(acopy) (LocalVariables|GetReturnedLines)) (Utilities|Array|Get(acopy) (LocalVariables|GetReturnedName)))
    (else
      (Widget|RemovefromParent (Variables|Default|GetDialogueWidgetRef))
      (Variables|Default|SetDialogueWidgetRef 0)
      (Variables|Default|SetLineCurrent 0)
      (bind _asbp_player_character (Utilities|Casting|CastToBP_PlayerCharacter (Game|GetPlayerCharacter 0)))
      (Pawn|Components|CharacterMovement|SetMovementMode (Variables|/Script/Engine.Character|GetCharacterMovement _asbp_player_character) "MOVE_Walking" 0))))