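; BP_BaseGameMode is a game mode that sets up input and UI when play begins.
; It sets game-and-UI input with the mouse locked to the viewport and the cursor visible, then adds a W_OpenLevel widget to the screen.
; On every level except M_Level01 it also creates W_HUD, stores it in the HUD variable and adds it to the viewport.
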(event EventBeginPlay
  (bind _returnvalue (Game|GetPlayerController 0))
  (Input|SetInputModeGameandUI _returnvalue 0 "LockAlways" false)
  (Variables|/Script/Engine.PlayerController|SetbShowMouseCursor _returnvalue true)
  (bind _returnvalue_2 (UserInterface|CreateWidget "/Game/UI/W_OpenLevel.W_OpenLevel_C"))
  (UserInterface|Viewport|AddtoViewport _returnvalue_2 0)
  (bind _returnvalue_3 (Game|GetCurrentLevelName true))
  (if (not (== _returnvalue_3 "M_Level01"))
    (bind _returnvalue_4 (UserInterface|CreateWidget "/Game/UI/HUD/W_HUD.W_HUD_C"))
    (bind _output_get (Variables|Default|SetHUD _returnvalue_4))
    (UserInterface|Viewport|AddtoViewport _output_get 0)))

(fn ConstructionScript)