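; Game instance Blueprint that restores saved player progress and audio settings when the game starts.
; On Init it loads the "Check" save slot, casts it to BP_SaveGame and copies its fields into its own variables.
; These cover sound volumes, player location, inventory counts such as arrows and money, and the saved weapon mesh and class.
; If the cast fails, nothing is copied.
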(event EventInit
  (bind _returnvalue (SaveGame|LoadGamefromSlot "Check"))
  (bind _asbp_save_game (Utilities|Casting|CastToBP_SaveGame _returnvalue))
  (Variables|Default|SetSavedMusicVolume (Variables|/Game/Blueprints/BP_SaveGame.BP_SaveGame_C|GetMusicSound _asbp_save_game))
  (Variables|Default|SetSavedSFXVolume (Variables|/Game/Blueprints/BP_SaveGame.BP_SaveGame_C|GetSFXSound _asbp_save_game))
  (Variables|Default|SetSavedUIVolume (Variables|/Game/Blueprints/BP_SaveGame.BP_SaveGame_C|GetUISound _asbp_save_game))
  (Variables|Default|SetSavedMasterVolume (Variables|/Game/Blueprints/BP_SaveGame.BP_SaveGame_C|GetMasterSound _asbp_save_game))
  (Variables|Default|SetPlayerLocation (Variables|/Game/Blueprints/BP_SaveGame.BP_SaveGame_C|GetPlayerLocation _asbp_save_game))
  (Variables|Default|SetArrows (Variables|/Game/Blueprints/BP_SaveGame.BP_SaveGame_C|GetArrows _asbp_save_game))
  (Variables|Default|SetMoney (Variables|/Game/Blueprints/BP_SaveGame.BP_SaveGame_C|GetMoney _asbp_save_game))
  (Variables|Default|SetPirogi (Variables|/Game/Blueprints/BP_SaveGame.BP_SaveGame_C|GetPirogi _asbp_save_game))
  (Variables|Default|SetLivingWater (Variables|/Game/Blueprints/BP_SaveGame.BP_SaveGame_C|GetLivingWater _asbp_save_game))
  (Variables|Default|SetCurrentWeaponMesh (Variables|/Game/Blueprints/BP_SaveGame.BP_SaveGame_C|GetSavedWeaponMesh _asbp_save_game))
  (Variables|Default|SetSavedWeaponClass (Variables|/Game/Blueprints/BP_SaveGame.BP_SaveGame_C|GetSavedWeaponClass _asbp_save_game)))