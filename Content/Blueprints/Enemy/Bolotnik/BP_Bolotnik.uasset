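; BP_Bolotnik is an enemy that turns its turret toward the player and plays sounds when damaged.
; Each tick it casts the player character and calls RotateTurret with the player's location while within a fixed range.
; On BeginPlay it binds a damage handler, which reads HealthComponent to choose between the hit and defeated sounds.
; No firing, health reduction or death logic appears in these graphs.
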(event Custom|TakeDamage
  (params (DamagedActor :type Actor%20Object%20Reference) (Damage :type Float%20%28single-precision%29) (DamageType :type Damage%20Type%20Object%20Reference) (InstigatedBy :type Controller%20Object%20Reference) (DamageCauser :type Actor%20Object%20Reference))
  (bind _returnvalue (Transformation|GetActorLocation))
  (if (<= (Variables|/Script/HAGJ.HealthComponent|GetHealth (Variables|Default|GetHealthComponent)) 0.0)
    (Audio|PlaySoundatLocation "/Game/Assets/Sound/SFX/SS/ss_defeated.ss_defeated" _returnvalue "0, 0, 0" 1.0 1.0 0.0 0 0 0)
    (else
      (Audio|PlaySoundatLocation "/Game/Assets/Sound/SFX/SS/ss_hit.ss_hit" _returnvalue "0, 0, 0" 1.0 1.0 0.0 0 0 0))))

(event EventBeginPlay
  (EventDispatchers|BindEventtoOnTakeAnyDamage (delegate Custom|TakeDamage)))

(event EventTick
  (params (DeltaSeconds :type Float%20%28single-precision%29))
  (bind _asbp_player_character (Utilities|Casting|CastToBP_PlayerCharacter (Game|GetPlayerCharacter 0)))
  (if (< (Math|Vector|Distance(Vector) (Transformation|GetActorLocation) (Transformation|GetActorLocation _asbp_player_character)) 1e+03)
    (Class|EnemyCharacter|RotateTurret (Transformation|GetActorLocation _asbp_player_character))))

(fn ConstructionScript
  (|CallParentFunction))