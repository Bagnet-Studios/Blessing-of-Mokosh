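; Enemy character Blueprint that tracks a health value and can award money to the player.
; On BeginPlay it seeds its current target health from the HealthComponent's maximum.
; Its AddMoney event casts player 0 to BP_PlayerCharacter and adds a small random reward, skipped once the balance nears a three-digit ceiling.
; The file does not call AddMoney itself.
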(event EventBeginPlay
  (Variables|Default|SetTargetHealthCurrent (Variables|/Script/HAGJ.HealthComponent|GetMaxHealth (Variables|Default|GetHealthComponent))))

(event EventAddMoney
  ;[1 1 1] Adding Money
  (bind _asbp_player_character (Utilities|Casting|CastToBP_PlayerCharacter (Game|GetPlayerCharacter 0)))
  (if (not (>= (Variables|/Game/Blueprints/Player/BP_PlayerCharacter.BP_PlayerCharacter_C|GetMoney _asbp_player_character) 989))
    (Variables|/Game/Blueprints/Player/BP_PlayerCharacter.BP_PlayerCharacter_C|SetMoney _asbp_player_character (+ (Math|Random|RandomIntegerinRange 3 10) (Variables|/Game/Blueprints/Player/BP_PlayerCharacter.BP_PlayerCharacter_C|GetMoney _asbp_player_character)))))

(fn ConstructionScript)