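; Auka character that gives way to a reward chest when the player hits it with a weapon.
; A capsule overlap with a BaseWeapon, while the player's WeaponComponent has CanAttack set, spawns a BP_Chest_ThirdSword nearby that grants Perun's Sword.
; It then toggles a W_Dialogue widget: an open one is removed, otherwise a new one shows briefly before Auka destroys itself.
; The SpawnChest guard is only set after the delay and destroy.
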(event OnComponentBeginOverlap(CapsuleComponent)
  (params (OverlappedComponent :type Primitive%20Component%20Object%20Reference) (OtherActor :type Actor%20Object%20Reference) (OtherComp :type Primitive%20Component%20Object%20Reference) (OtherBodyIndex :type Integer) (bFromSweep :type Boolean) (SweepResult :type Hit%20Result%20Structure%20%28by%20ref%29))
  (bind _returnvalue (Transformation|GetActorTransform))
  (Utilities|Casting|CastToBaseWeapon OtherActor)
  (bind _asbp_player_character (Utilities|Casting|CastToBP_PlayerCharacter (Game|GetPlayerCharacter 0)))
  (if (Variables|/Script/HAGJ.WeaponComponent|GetbCanAttack (Variables|/Script/HAGJ.BaseCharacter|GetWeaponComponent _asbp_player_character))
    (if (not (Variables|Default|GetSpawnChest))
      (Game|SpawnActorfromClass "/Game/Blueprints/Environment/Chests/BP_Chest_ThirdSword.BP_Chest_ThirdSword_C" (Math|Transform|MakeTransform (Math|Vector|MakeVector (+ (.x (.location _returnvalue)) 1e+02) (.y (.location _returnvalue)) (- (.z (.location _returnvalue)) 88.0)) (Math|Rotator|MakeRotator (.roll (Transformation|GetWorldRotation (Variables|/Script/HAGJ.PlayerCharacter|GetCameraComponent _asbp_player_character))) (+ (.pitch (Transformation|GetWorldRotation (Variables|/Script/HAGJ.PlayerCharacter|GetCameraComponent _asbp_player_character))) 4e+01) (.yaw (Transformation|GetWorldRotation (Variables|/Script/HAGJ.PlayerCharacter|GetCameraComponent _asbp_player_character))))) "AdjustIfPossibleButAlwaysSpawn" 0 "/Game/Blueprints/Weapons/BP_ThirdSword.BP_ThirdSword_C" "You’ve got the Perun’s Sword now!" false 0)
      (Utilities|IsValid (Variables|Default|GetDialog)
        (:Is%20Valid
          (Widget|RemovefromParent (Variables|Default|GetDialog))
          (Variables|Default|SetDialog 0))
        (:Is%20Not%20Valid
          (bind _returnvalue_2 (UserInterface|CreateWidget "/Game/UI/W_Dialogue.W_Dialogue_C" (Game|GetPlayerController 0)))
          (bind _output_get (Variables|Default|SetDialog _returnvalue_2))
          (UserInterface|Viewport|AddtoViewport _output_get 0)
          (Variables|/Game/UI/W_Dialogue.W_Dialogue_C|SetDialogueText (Variables|Default|GetDialog) (Variables|Default|GetTEXT))
          (Utilities|FlowControl|Delay 0.5)
          (Widget|RemovefromParent (Variables|Default|GetDialog))
          (Variables|Default|SetDialog 0)
          (Actor|DestroyActor)
          (Variables|Default|SetSpawnChest true))))))

(fn ConstructionScript)