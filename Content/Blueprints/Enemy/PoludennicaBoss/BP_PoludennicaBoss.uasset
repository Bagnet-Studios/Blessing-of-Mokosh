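; Poludnitsa (noonwraith) boss enemy Blueprint that adds an intro line, combat audio and a money reward.
; The first Sphere overlap by any actor shows a W_Dialogue taunt for five seconds through DoOnce.
; Damage plays a hit sound, or a defeat sound while deactivating AttackCollision once HealthComponent health is depleted.
; AddMoney grants the player a fixed 50, via an equal-bound random range, unless their money nears the cap.
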(event OnComponentBeginOverlap(Sphere)
  (params (OverlappedComponent :type Primitive%20Component%20Object%20Reference) (OtherActor :type Actor%20Object%20Reference) (OtherComp :type Primitive%20Component%20Object%20Reference) (OtherBodyIndex :type Integer) (bFromSweep :type Boolean) (SweepResult :type Hit%20Result%20Structure%20%28by%20ref%29))
  (Utilities|FlowControl|DoOnce false
    (:Completed
      (bind _returnvalue (UserInterface|CreateWidget "/Game/UI/W_Dialogue.W_Dialogue_C"))
      (Variables|Default|SetDialogue%20widget _returnvalue)
      (Variables|/Game/UI/W_Dialogue.W_Dialogue_C|SetDialogueText (Variables|Default|GetDialogue%20widget) "Tell me, brave hero, am I beautiful? Will you stay with me?!")
      (Variables|/Game/UI/W_Dialogue.W_Dialogue_C|SetName (Variables|Default|GetDialogue%20widget) "Poludnitsa ")
      (UserInterface|Viewport|AddtoViewport (Variables|Default|GetDialogue%20widget) 0)
      (Utilities|FlowControl|Delay 5.0)
      (Widget|RemovefromParent (Variables|Default|GetDialogue%20widget))
      (Variables|Default|SetDialogue%20widget 0))))

(event Custom|Destroyed
  (params (DestroyedActor :type Actor%20Object%20Reference)))

(event Custom|TakeDamage
  (params (DamagedActor :type Actor%20Object%20Reference) (Damage :type Float%20%28single-precision%29) (DamageType :type Damage%20Type%20Object%20Reference) (InstigatedBy :type Controller%20Object%20Reference) (DamageCauser :type Actor%20Object%20Reference))
  (bind _returnvalue (Transformation|GetActorLocation))
  (if (<= (Variables|/Script/HAGJ.HealthComponent|GetHealth (Variables|Default|GetHealthComponent)) 0.0)
    (Audio|PlaySoundatLocation "/Game/Assets/Sound/SFX/Noonwraith/noonwraith_defeated.noonwraith_defeated" _returnvalue "0, 0, 0" 1.0 1.0 0.0 0 0 0)
    (Components|Activation|SetActive (Variables|Default|GetAttackCollision) false false)
    (else
      (Audio|PlaySoundatLocation "/Game/Assets/Sound/SFX/Noonwraith/noonwraith_hit_new.noonwraith_hit_new" _returnvalue "0, 0, 0" 1.0 1.0 0.0 0 0 0))))

(event EventAddMoney
  (bind _asbp_player_character (Utilities|Casting|CastToBP_PlayerCharacter (Game|GetPlayerCharacter 0)))
  (if (not (>= (Variables|/Game/Blueprints/Player/BP_PlayerCharacter.BP_PlayerCharacter_C|GetMoney _asbp_player_character) 989))
    (Variables|/Game/Blueprints/Player/BP_PlayerCharacter.BP_PlayerCharacter_C|SetMoney _asbp_player_character (+ (Math|Random|RandomIntegerinRange 50 50) (Variables|/Game/Blueprints/Player/BP_PlayerCharacter.BP_PlayerCharacter_C|GetMoney _asbp_player_character)))))

(event EventBeginPlay
  (Game|BindEventtoOnDestroyed (delegate Custom|Destroyed))
  (EventDispatchers|BindEventtoOnTakeAnyDamage (delegate Custom|TakeDamage)))

(fn ConstructionScript
  (|CallParentFunction))