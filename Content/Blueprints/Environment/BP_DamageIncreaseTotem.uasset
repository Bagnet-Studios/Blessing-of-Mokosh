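; BP_DamageIncreaseTotem is an interactable environment totem that greatly boosts the player's weapon damage.
; On Interact, it multiplies the DamageMultiplier on the PlayerRef's WeaponComponent by a hundredfold and prints the new value.
; The graph has no use limit or reset, so repeated interactions compound the boost.
; BeginPlay and the construction script only call their parent implementations.
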(event EventBeginPlay
  (|CallParentFunction))

(event EventInteract
  (bind _playerref (Variables|Default|GetPlayerRef))
  (bind _weaponcomponent (Variables|/Script/HAGJ.BaseCharacter|GetWeaponComponent _playerref))
  (bind _output_get (Variables|/Script/HAGJ.WeaponComponent|SetDamageMultiplier _weaponcomponent (* (Variables|/Script/HAGJ.WeaponComponent|GetDamageMultiplier _weaponcomponent) 1e+02)))
  (Development|PrintString (Utilities|String|ToString(Float) _output_get)))

(fn ConstructionScript
  (|CallParentFunction))