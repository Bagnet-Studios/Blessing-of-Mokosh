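; Checkpoint trigger that saves game progress when anything overlaps its box, playing a sound.
; It copies player 0's location, inventory, weapon and opened chests, plus volume settings from the game instance, into local variables.
; A second sequence step writes them to the "Check" slot, updating the existing BP_SaveGame or creating one.
; The overlapping actor is never checked, and the fire emitter spawn is unconnected.
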(event OnComponentBeginOverlap(Box)
  (params (OverlappedComponent :type Primitive%20Component%20Object%20Reference) (OtherActor :type Actor%20Object%20Reference) (OtherComp :type Primitive%20Component%20Object%20Reference) (OtherBodyIndex :type Integer) (bFromSweep :type Boolean) (SweepResult :type Hit%20Result%20Structure%20%28by%20ref%29))
  (Audio|PlaySound2D "/Game/Assets/Sound/UI/Holy.Holy" 1.0 1.0 0.0 0 0)
  (Utilities|FlowControl|Sequence
    (:then_0
      (bind _asbp_player_character (Utilities|Casting|CastToBP_PlayerCharacter (Game|GetPlayerCharacter 0)))
      (bind _asbp_default_game_instance (Utilities|Casting|CastToBP_DefaultGameInstance (Game|GetGameInstance)))
      (Variables|Default|SetPlayerLocation (Transformation|GetActorLocation _asbp_player_character))
      (Variables|Default|SetPlayerMoney (Variables|/Game/Blueprints/Player/BP_PlayerCharacter.BP_PlayerCharacter_C|GetMoney _asbp_player_character))
      (Variables|Default|SetPlayerArrows (Variables|/Script/HAGJ.BaseCharacter|GetArrowCount _asbp_player_character))
      (Variables|Default|SetMaster (Variables|/Game/Blueprints/BP_DefaultGameInstance.BP_DefaultGameInstance_C|GetSavedMasterVolume _asbp_default_game_instance))
      (Variables|Default|SetMusic (Variables|/Game/Blueprints/BP_DefaultGameInstance.BP_DefaultGameInstance_C|GetSavedMusicVolume _asbp_default_game_instance))
      (Variables|Default|SetSFX (Variables|/Game/Blueprints/BP_DefaultGameInstance.BP_DefaultGameInstance_C|GetSavedSFXVolume _asbp_default_game_instance))
      (Variables|Default|SetUI (Variables|/Game/Blueprints/BP_DefaultGameInstance.BP_DefaultGameInstance_C|GetSavedUIVolume _asbp_default_game_instance))
      (Variables|Default|SetPlayerPirogi (Variables|/Script/HAGJ.BaseCharacter|GetPie _asbp_player_character))
      (Variables|Default|SetPlayerLivingWater (Variables|/Script/HAGJ.BaseCharacter|GetLivingWater _asbp_player_character))
      (Variables|Default|SetCurrentWeapon (Variables|/Game/Blueprints/Player/BP_PlayerCharacter.BP_PlayerCharacter_C|GetCurrentWeaponMesh _asbp_player_character))
      (Variables|Default|SetWeaponClass (Variables|/Game/Blueprints/Player/BP_PlayerCharacter.BP_PlayerCharacter_C|GetWeaponClass _asbp_player_character))
      (Variables|Default|SetOpenedChests (Variables|/Game/Blueprints/Player/BP_PlayerCharacter.BP_PlayerCharacter_C|GetOpenedChests _asbp_player_character)))
    (:then_1
      (bind _returnvalue (SaveGame|DoesSaveGameExist "Check"))
      (if _returnvalue
        (bind _returnvalue_2 (SaveGame|LoadGamefromSlot "Check"))
        (bind _asbp_save_game (Utilities|Casting|CastToBP_SaveGame _returnvalue_2))
        (Variables|/Game/Blueprints/BP_SaveGame.BP_SaveGame_C|SetPlayerLocation _asbp_save_game (Variables|Default|GetPlayerLocation))
        (Variables|/Game/Blueprints/BP_SaveGame.BP_SaveGame_C|SetArrows _asbp_save_game (Variables|Default|GetPlayerArrows))
        (Variables|/Game/Blueprints/BP_SaveGame.BP_SaveGame_C|SetMoney _asbp_save_game (Variables|Default|GetPlayerMoney))
        (Variables|/Game/Blueprints/BP_SaveGame.BP_SaveGame_C|SetMasterSound _asbp_save_game (Variables|Default|GetMaster))
        (Variables|/Game/Blueprints/BP_SaveGame.BP_SaveGame_C|SetMusicSound _asbp_save_game (Variables|Default|GetMusic))
        (Variables|/Game/Blueprints/BP_SaveGame.BP_SaveGame_C|SetSFXSound _asbp_save_game (Variables|Default|GetSFX))
        (Variables|/Game/Blueprints/BP_SaveGame.BP_SaveGame_C|SetUISound _asbp_save_game (Variables|Default|GetUI))
        (Variables|/Game/Blueprints/BP_SaveGame.BP_SaveGame_C|SetPirogi _asbp_save_game (Variables|Default|GetPlayerPirogi))
        (Variables|/Game/Blueprints/BP_SaveGame.BP_SaveGame_C|SetLivingWater _asbp_save_game (Variables|Default|GetPlayerLivingWater))
        (Variables|/Game/Blueprints/BP_SaveGame.BP_SaveGame_C|SetSavedWeaponMesh _asbp_save_game (Variables|Default|GetCurrentWeapon))
        (Variables|/Game/Blueprints/BP_SaveGame.BP_SaveGame_C|SetSavedWeaponClass _asbp_save_game (Variables|Default|GetWeaponClass))
        (Variables|/Game/Blueprints/BP_SaveGame.BP_SaveGame_C|SetSavedOpenedChests _asbp_save_game (Variables|Default|GetOpenedChests))
        (SaveGame|SaveGametoSlot _asbp_save_game "Check")
        (else
          (bind _returnvalue_3 (SaveGame|CreateSaveGameObject "/Game/Blueprints/BP_SaveGame.BP_SaveGame_C"))
          (Variables|/Game/Blueprints/BP_SaveGame.BP_SaveGame_C|SetPlayerLocation _returnvalue_3 (Variables|Default|GetPlayerLocation))
          (Variables|/Game/Blueprints/BP_SaveGame.BP_SaveGame_C|SetArrows _returnvalue_3 (Variables|Default|GetPlayerArrows))
          (Variables|/Game/Blueprints/BP_SaveGame.BP_SaveGame_C|SetMoney _returnvalue_3 (Variables|Default|GetPlayerMoney))
          (Variables|/Game/Blueprints/BP_SaveGame.BP_SaveGame_C|SetMasterSound _returnvalue_3 (Variables|Default|GetMaster))
          (Variables|/Game/Blueprints/BP_SaveGame.BP_SaveGame_C|SetMusicSound _returnvalue_3 (Variables|Default|GetMusic))
          (Variables|/Game/Blueprints/BP_SaveGame.BP_SaveGame_C|SetSFXSound _returnvalue_3 (Variables|Default|GetSFX))
          (Variables|/Game/Blueprints/BP_SaveGame.BP_SaveGame_C|SetUISound _returnvalue_3 (Variables|Default|GetUI))
          (Variables|/Game/Blueprints/BP_SaveGame.BP_SaveGame_C|SetPirogi _returnvalue_3 (Variables|Default|GetPlayerPirogi))
          (Variables|/Game/Blueprints/BP_SaveGame.BP_SaveGame_C|SetLivingWater _returnvalue_3 (Variables|Default|GetPlayerLivingWater))
          (Variables|/Game/Blueprints/BP_SaveGame.BP_SaveGame_C|SetSavedWeaponMesh _returnvalue_3 (Variables|Default|GetCurrentWeapon))
          (Variables|/Game/Blueprints/BP_SaveGame.BP_SaveGame_C|SetSavedWeaponClass _returnvalue_3 (Variables|Default|GetWeaponClass))
          (Variables|/Game/Blueprints/BP_SaveGame.BP_SaveGame_C|SetSavedOpenedChests _returnvalue_3 (Variables|Default|GetOpenedChests))
          (SaveGame|SaveGametoSlot _returnvalue_3 "Check"))))))

(fn ConstructionScript)