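; Base weapon chest actor that, when interacted with while closed, spawns a spark effect and gives the player its configured weapon through their WeaponComponent.
; Opening also adds a HUD widget, disables the box collision, shows text and registers the chest in the player's OpenedChests.
; A timeline rotates the lid mesh, which then simulates physics before the text hides after a delay.
; Chests already marked opened replay that animation shortly after BeginPlay.
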(event EventInteract
  (bind _cube1 (Variables|Default|GetCube1))
  (if (not (Variables|Default|GetbIsOpened))
    (Niagara|SpawnSystematLocation "/Game/Assets/FX/N_Spark_System.N_Spark_System" (Transformation|GetActorLocation))
    (bind _asbp_player_character (Utilities|Casting|CastToBP_PlayerCharacter (Game|GetPlayerCharacter 0)))
    (bind _output_get (Variables|Default|SetPlayerRef _asbp_player_character))
    (Variables|/Script/HAGJ.WeaponComponent|SetWeaponClass (Variables|/Script/HAGJ.BaseCharacter|GetWeaponComponent _output_get) 0)
    (Variables|/Script/HAGJ.WeaponComponent|SetWeaponClass (Variables|/Script/HAGJ.BaseCharacter|GetWeaponComponent _output_get) (Variables|Default|GetWeaponToGive))
    (Class|WeaponComponent|SpawnWeapon (Variables|/Script/HAGJ.BaseCharacter|GetWeaponComponent _output_get))
    (bind _returnvalue (UserInterface|CreateWidget "/Game/UI/HUD/W_HUD.W_HUD_C"))
    (UserInterface|Viewport|AddtoViewport _returnvalue 0)
    (Collision|SetCollisionEnabled (Variables|Default|GetBox) "NoCollision")
    (Rendering|SetVisibility (Variables|Default|GetTextRender) true false)
    (Variables|Default|SetbIsOpened true)
    (Utilities|Array|Add (Variables|/Game/Blueprints/Player/BP_PlayerCharacter.BP_PlayerCharacter_C|GetOpenedChests (Variables|Default|GetPlayerRef)) self)
    (Variables|/Game/Blueprints/Player/BP_PlayerCharacter.BP_PlayerCharacter_C|SetWeaponClass (Variables|Default|GetPlayerRef) (Variables|Default|GetWeaponToGive))
    (bind _time (Timeline|Timeline_0 Play)
      (:Update
        (Transformation|SetWorldRotation _cube1 (Math|Rotator|Lerp(Rotator) (Transformation|GetWorldRotation _cube1) "-100.000000, 0,10.000000" _time true) false false))
      (:Finished
        (Physics|SetSimulatePhysics _cube1 true)
        (Utilities|FlowControl|Delay 1e+01)
        (Rendering|SetVisibility (Variables|Default|GetTextRender) false false)))))

(event EventBeginPlay
  (bind _cube1 (Variables|Default|GetCube1))
  (Utilities|FlowControl|Delay 0.2)
  (if (Variables|Default|GetbIsOpened)
    (bind _time (Timeline|Timeline_1 PlayFromStart)
      (:Update
        (Transformation|SetWorldRotation _cube1 (Math|Rotator|Lerp(Rotator) (Transformation|GetWorldRotation _cube1) "-100.000000, 0,10.000000" _time true) false false))
      (:Finished
        (Physics|SetSimulatePhysics _cube1 true)
        (Utilities|FlowControl|Delay 1e+01)
        (Rendering|SetVisibility (Variables|Default|GetTextRender) false false)))))

(fn ConstructionScript)