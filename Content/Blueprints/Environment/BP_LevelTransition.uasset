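; Level exit trigger that gates travel to another level on whether the player holds a weapon.
; On overlap of component A, it checks player 0's current weapon: if valid, it shows a W_CloseLevel widget and passes it the destination level name.
; Otherwise it shows a "Talk with Dad" dialogue widget, which is removed when the overlap ends.
; The overlapping actor itself is not checked.
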(event OnComponentBeginOverlap(a)
  (params (OverlappedComponent :type Primitive%20Component%20Object%20Reference) (OtherActor :type Actor%20Object%20Reference) (OtherComp :type Primitive%20Component%20Object%20Reference) (OtherBodyIndex :type Integer) (bFromSweep :type Boolean) (SweepResult :type Hit%20Result%20Structure%20%28by%20ref%29))
  (bind _asbp_player_character (Utilities|Casting|CastToBP_PlayerCharacter (Game|GetPlayerCharacter 0)))
  (Variables|/Script/HAGJ.WeaponComponent|GetCurrentWeapon (Variables|/Script/HAGJ.BaseCharacter|GetWeaponComponent _asbp_player_character)
    (:then
      (bind _returnvalue (UserInterface|CreateWidget "/Game/UI/W_CloseLevel.W_CloseLevel_C"))
      (bind _output_get (Variables|Default|SetClose%20level%20widget%20ref _returnvalue))
      (UserInterface|Viewport|AddtoViewport _returnvalue 0)
      (Variables|/Game/UI/W_CloseLevel.W_CloseLevel_C|SetLevel%20Name _output_get (Variables|Default|GetTo%20level%20name)))
    (:else
      (bind _returnvalue_2 (UserInterface|CreateWidget "/Game/UI/W_Dialogue.W_Dialogue_C"))
      (Variables|/Game/UI/W_Dialogue.W_Dialogue_C|SetDialogueText _returnvalue_2 "Talk with Dad")
      (UserInterface|Viewport|AddtoViewport _returnvalue_2 0))))

(event OnComponentEndOverlap(a)
  (params (OverlappedComponent :type Primitive%20Component%20Object%20Reference) (OtherActor :type Actor%20Object%20Reference) (OtherComp :type Primitive%20Component%20Object%20Reference) (OtherBodyIndex :type Integer))
  (Widget|RemovefromParent (stale OnComponentBeginOverlap(a) _returnvalue_2)))

(fn ConstructionScript)