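; Interactable chest that swaps the player's current weapon for a second weapon.
; Interact spawns an effect, detaches the held weapon mesh, then assigns the chest's weapon class to the player's WeaponComponent and spawns it.
; It disables the box collision and shows a text label while a timeline rotates a cube open like a lid.
; The cube then switches to physics simulation, and the text hides after a delay.
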(event EventInteract
  (bind _cube1 (Variables|Default|GetCube1))
  (bind _playerref (Variables|Default|GetPlayerRef))
  (bind _weaponcomponent (Variables|/Script/HAGJ.BaseCharacter|GetWeaponComponent _playerref))
  (Niagara|SpawnSystematLocation 0 "0, 0, 0")
  (Transformation|DetachFromComponent (Variables|/Script/HAGJ.BaseWeapon|GetWeaponMesh (Variables|/Script/HAGJ.WeaponComponent|GetCurrentWeapon _weaponcomponent)) "KeepRelative" "KeepRelative" "KeepRelative" true)
  (Variables|/Script/HAGJ.WeaponComponent|SetWeaponClass _weaponcomponent 0)
  (Variables|/Script/HAGJ.WeaponComponent|SetWeaponClass _weaponcomponent (Variables|Default|GetWeapon%20Class))
  (Class|WeaponComponent|SpawnWeapon _weaponcomponent)
  (Collision|SetCollisionEnabled (Variables|Default|GetBox) "NoCollision")
  (Rendering|SetVisibility (Variables|Default|GetTextRender) true false)
  (bind _time (Timeline|Timeline_0 Play)
    (:Update
      (Transformation|SetWorldRotation _cube1 (Math|Rotator|Lerp(Rotator) (Transformation|GetWorldRotation _cube1) "-100.000000, 0,10.000000" _time true) false false))
    (:Finished
      (Physics|SetSimulatePhysics _cube1 true)
      (Utilities|FlowControl|Delay 1e+01)
      (Rendering|SetVisibility (Variables|Default|GetTextRender) false false))))

(fn ConstructionScript
  (|CallParentFunction))