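; BP_DamageIncreaseTotem is an interactable environment totem that buffs the player's damage.
; On Interact it doubles the DamageMultiplier on the player's WeaponComponent and disables its Box collision.
; It shows its TextRender for ten seconds, then hides only the text; the damage buff is never reverted here.
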(event EventInteract
  (bind _playerref (Variables|Default|GetPlayerRef))
  (bind _textrender (Variables|Default|GetTextRender))
  (bind _weaponcomponent (Variables|/Script/HAGJ.BaseCharacter|GetWeaponComponent _playerref))
  (Development|PrintString "damage buffed")
  (Variables|/Script/HAGJ.WeaponComponent|SetDamageMultiplier _weaponcomponent (* (Variables|/Script/HAGJ.WeaponComponent|GetDamageMultiplier _weaponcomponent) 2.0))
  (Collision|SetCollisionEnabled (Variables|Default|GetBox) "NoCollision")
  (Rendering|SetVisibility _textrender true false)
  (Utilities|FlowControl|Delay 1e+01)
  (Rendering|SetVisibility _textrender false false))

(fn ConstructionScript
  (|CallParentFunction))