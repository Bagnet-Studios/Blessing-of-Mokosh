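; Legacy top-down player character that faces the cursor, moves on world axes, dashes, eats pies to heal, interacts with overlapping actors and spends money.
; Tick cursor traces drive rotation and the enemy target widget.
; Fireball and AoE spawn ability actors whose cast events drive one shared cooldown and the action-slot widget; movement input interrupts casts.
; Destruction unpossesses and shows the death screen; H self-destructs, and inventory-camera logic is unwired.
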(event Custom|Rofl
  (params (DestroyedActor :type Actor%20Object%20Reference))
  (Pawn|UnPossess (Game|GetPlayerController 0))
  (bind _returnvalue (UserInterface|CreateWidget "/Game/UI/W_Death.W_Death_C"))
  (UserInterface|Viewport|AddtoViewport _returnvalue 0))

(event Custom|StartCooldown
  ;[1 1 1] Spells
  (bind _returnvalue (Utilities|Time|SetTimerbyEvent (delegate Custom|EndCooldown) (.cooldowntime (.AbilityDetails (Utilities|GetClassDefaults (stale Input|ActionEvents|InputActionSpellFireBall _output_get))))))
  (bind _output_get (Variables|Default|SetCooldownTimer _returnvalue)))

(event Custom|EndCooldown
  ;[1 1 1] Spells
  (Variables|Default|SetbCanCastSpell true)
  (Default|UpdateAppearance (Variables|Default|GetActionSlot) (Variables|Default|GetbCanCastSpell))
  (Utilities|Time|ClearandInvalidateTimerbyHandle (stale Custom|StartCooldown _output_get)))

(event Custom|StartCooldown_2
  ;[1 1 1] Spells
  (bind _returnvalue (Utilities|Time|SetTimerbyEvent (delegate Custom|EndCooldown_2) (.cooldowntime (.AbilityDetails (Utilities|GetClassDefaults (stale Input|ActionEvents|InputActionSpellAOE _output_get))))))
  (bind _output_get (Variables|Default|SetCooldownTimer _returnvalue)))

(event Custom|EndCooldown_2
  ;[1 1 1] Spells
  (Variables|Default|SetbCanCastSpell true)
  (Default|UpdateAppearance (Variables|Default|GetActionSlot) (Variables|Default|GetbCanCastSpell))
  (Utilities|Time|ClearandInvalidateTimerbyHandle (stale Custom|StartCooldown_2 _output_get)))

(event EventBeginPlay
  (Game|BindEventtoOnDestroyed (delegate Custom|Rofl))
  ;[1 1 1] Set initial max speed
  (Variables|/Script/Engine.CharacterMovementComponent|SetMaxWalkSpeed (Variables|Character|GetCharacterMovement) 8e+02)
  (bind _returnvalue (UserInterface|CreateWidget "/Game/UI/ActionBar/W_ActionSlot.W_ActionSlot_C" 0 0))
  (Variables|Default|SetActionSlot _returnvalue))

(event EventTick
  (params (DeltaSeconds :type Float%20%28single-precision%29))
  (bind _returnvalue (Game|GetPlayerController 0))
  (bind _hitresult (Game|Player|GetHitResultUnderCursorbyChannel _returnvalue "TraceTypeQuery1" true))
  (bind (_bblockinghit _binitialoverlap _time _distance _location _impactpoint _normal _impactnormal _physmat _hitactor) (Collision|BreakHitResult _hitresult))
  ;[1 1 1] Set rotate to cursor
  (Transformation|SetActorRotation (Math|Rotator|MakeRotator 0.0 0.0 (.Yaw (Math|Rotator|BreakRotator (Math|Rotator|FindLookatRotation (Transformation|GetActorLocation) _impactpoint)))))
  ;[1 1 1] Show Enemy Health bar
  (bind _output_get (Variables|Default|SetHit%20Actor _hitactor))
  (Utilities|Casting|CastToBP_EnemyCharacter _output_get
    (:then
      (Variables|Default|GetEnemy%20widget
        (:then)
        (:else
          (bind _returnvalue_2 (UserInterface|CreateWidget "/Game/UI/W_TargetUI.W_TargetUI_C"))
          (bind _output_get_2 (Variables|Default|SetEnemy%20widget _returnvalue_2))
          (UserInterface|Viewport|AddtoViewport _output_get_2 0))))
    (:CastFailed
      (bind _enemy_widget (Variables|Default|GetEnemy%20widget)
        (:then
          (Widget|RemovefromParent _enemy_widget)
          (Variables|Default|SetEnemy%20widget 0))
        (:else)))))

(event Input|ActionEvents|InputActionEatPirozhok
  (params (Key :type Key%20Structure))
  (bind _healthcomponent (Variables|Default|GetHealthComponent))
  ;[1 1 1] Eat Heal
  (:Pressed
    (if (not (== (Variables|Default|GetPie) 0))
      (bind _result (Math|Integer|DecrementInt (Variables|Default|GetPie))
        (:%20%20
          (Variables|Default|SetPie _result)
          (Variables|/Script/HAGJ.HealthComponent|SetHealth _healthcomponent (+ (Variables|/Script/HAGJ.HealthComponent|GetHealth _healthcomponent) 5.0)))))))

(event Input|ActionEvents|InputActionInventory
  (params (Key :type Key%20Structure))
  ;[1 0 0] Open Inventary
)

(event Input|ActionEvents|InputActionDash
  (params (Key :type Key%20Structure))
  (bind _charactermovement (Variables|Character|GetCharacterMovement))
  ;[1 1 1] Dsh
  (:Pressed
    (if (Variables|Default|GetbCanDash)
      (Variables|Default|SetbCanDash false)
      (Variables|/Script/Engine.CharacterMovementComponent|SetMaxWalkSpeed _charactermovement 1.5e+03)
      (Utilities|FlowControl|Delay 0.3)
      (Variables|/Script/Engine.CharacterMovementComponent|SetMaxWalkSpeed _charactermovement 6e+02)
      (Utilities|FlowControl|Delay 2.0)
      (Variables|Default|SetbCanDash true))))

(event Input|ActionEvents|InputActionSpellAOE
  (params (Key :type Key%20Structure))
  ;[1 1 1] Spells
  (:Pressed
    (if (Variables|Default|GetbCanCastSpell)
      (Audio|PlaySoundatLocation 0 (Transformation|GetActorLocation) "0, 0, 0" 1.0 1.0 0.0 0 0 0)
      (bind _output_get (Variables|Default|SetAbility%20Class "/Game/Blueprints/AbilitySystem/AOE/BP_HolyGround_AoE.BP_HolyGround_AoE_C"))
      (bind _returnvalue (Game|SpawnActorfromClass _output_get (Transformation|GetActorTransform (Game|GetPlayerCharacter 0)) "Undefined" 0 (Game|GetPlayerCharacter 0) 0))
      (Variables|Default|SetbCanCastSpell false)
      (EventDispatchers|BindEventtoCastSuccess _returnvalue (delegate Custom|StartCooldown_2))
      (EventDispatchers|BindEventtoCastInterrupted _returnvalue (delegate Custom|EndCooldown_2))
      (Default|UpdateAppearance (Variables|Default|GetActionSlot) (Variables|Default|GetbCanCastSpell)))))

(event Input|ActionEvents|InputActionSpellFireBall
  (params (Key :type Key%20Structure))
  ;[1 1 1] Spells
  (:Pressed
    (if (Variables|Default|GetbCanCastSpell)
      (Audio|PlaySoundatLocation "/Game/Assets/Sound/SFX/Ignition.Ignition" (Transformation|GetActorLocation) "0, 0, 0" 1.0 1.0 0.0 0 0 0)
      (bind _output_get (Variables|Default|SetAbility%20Class "/Game/Blueprints/AbilitySystem/Projectiles/Fireball/BP_Fireball_Ability.BP_Fireball_Ability_C"))
      (bind _returnvalue (Game|SpawnActorfromClass _output_get (Transformation|GetActorTransform (Game|GetPlayerCharacter 0)) "Undefined" 0 (Game|GetPlayerCharacter 0) 0))
      (Variables|Default|SetbCanCastSpell false)
      (EventDispatchers|BindEventtoCastSuccess _returnvalue (delegate Custom|StartCooldown))
      (EventDispatchers|BindEventtoCastInterrupted _returnvalue (delegate Custom|EndCooldown))
      (Default|UpdateAppearance (Variables|Default|GetActionSlot) (Variables|Default|GetbCanCastSpell)))))

(event Input|ActionEvents|InputActionPause
  (params (Key :type Key%20Structure))
  ;[1 1 1] Pause
  (:Pressed
    (bind _returnvalue (UserInterface|CreateWidget "/Game/UI/HUD/W_Pause.W_Pause_C"))
    (UserInterface|Viewport|AddtoViewport _returnvalue 0)))

(event Input|ActionEvents|InputActionInteract
  (params (Key :type Key%20Structure))
  ;[1 1 1] Interact with NPC
  (:Pressed
    (bind _outactors (Actor|GetAllActorswithInterface "/Game/Blueprints/Interfases/Interact_I.Interact_I_C"))
    (for _array_element _outactors
      (if (Collision|IsOverlappingActor _array_element self :!class /Script/Engine.Actor)
        (Class|InteractI|Interact(Message) _array_element)))))

(event Input|AxisEvents|InputAxisMoveForward
  (params (AxisValue :type Float%20%28single-precision%29))
  ;[1 1 1] Movement
  (Pawn|Input|AddMovementInput (Math|Vector|GetForwardVector "0, 0, 0") AxisValue false)
  (if (or (!= AxisValue 0.0) (!= (stale Input|AxisEvents|InputAxisMoveRight AxisValue) 0.0))
    (Default|CallInterruptCast)))

(event Input|AxisEvents|InputAxisMoveRight
  (params (AxisValue :type Float%20%28single-precision%29))
  ;[1 1 1] Movement
  (Pawn|Input|AddMovementInput (Math|Vector|GetRightVector "0, 0, 0") AxisValue false)
  (if (or (!= (stale Input|AxisEvents|InputAxisMoveForward AxisValue) 0.0) (!= AxisValue 0.0))
    (Default|CallInterruptCast)))

(event Input|KeyboardEvents|H
  (params (Key :type Key%20Structure))
  (:Pressed
    (Components|DestroyComponent (Variables|Default|GetWeaponComponent))
    (Actor|DestroyActor)))

(fn ConstructionScript)

(fn SpendMoney
  (params (Decrease%20Money :type Integer))
  (bind _output_get (Variables|Default|SetMoney (- (Variables|Default|GetMoney) Decrease%20Money)))
  (return _output_get))