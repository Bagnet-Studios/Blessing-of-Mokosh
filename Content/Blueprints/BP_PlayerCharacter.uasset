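; Player character Blueprint for a cursor-aimed game with world-axis movement, a cooldown-gated dash, NPC interaction and money spending.
; A custom event yaws the character toward the cursor's trace hit, Tick draws a debug line there, and movement input calls an interrupt on casting.
; Interact messages overlapping actors that implement Interact_I.
; Inventory blends to a child-actor camera, then opens a widget in UI-only mode.
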(event EventBeginPlay
  (Variables|/Script/Engine.CharacterMovementComponent|SetMaxWalkSpeed (Variables|Character|GetCharacterMovement) 8e+02))

(event EventRotateCharactertoCursor
  (Transformation|SetActorRotation (Math|Rotator|MakeRotator 0.0 0.0 (.Yaw (Math|Rotator|BreakRotator (Math|Rotator|FindLookatRotation (Transformation|GetActorLocation) (.ImpactPoint (Collision|BreakHitResult (.HitResult (Game|Player|GetHitResultUnderCursorbyChannel (Game|GetPlayerController 0) "TraceTypeQuery1" true))))))))))

(event EventTick
  (params (DeltaSeconds :type Float%20%28single-precision%29))
  (Rendering|Debug|DrawDebugLine (Transformation|GetActorLocation) (.ImpactPoint (Collision|BreakHitResult (.HitResult (Game|Player|GetHitResultUnderCursorbyChannel (Game|GetPlayerController 0) "TraceTypeQuery1" true)))) "(R=0.411458,G=0.029545,B=0.087083,A=1.000000)" 0.0 5.0))

(event Input|ActionEvents|InputActionInteract
  (params (Key :type Key%20Structure :default "None"))
  ;[1 1 1] Interact with NPC
  (:Pressed
    (bind _outactors (Actor|GetAllActorswithInterface "/Game/Dialogue/Interact_I.Interact_I_C"))
    (for _array_element _outactors
      (if (Collision|IsOverlappingActor _array_element self :!class /Script/Engine.Actor)
        (Class|InteractI|Interact(Message) _array_element)))))

(event Input|ActionEvents|InputActionInventory
  (params (Key :type Key%20Structure :default "None"))
  (bind _returnvalue (Game|GetPlayerController 0))
  (:Pressed
    (Game|Player|SetViewTargetwithBlend (Game|GetPlayerController 0) (Variables|/Script/Engine.ChildActorComponent|GetChildActor (Variables|Default|GetInventoryCamera)) 2.0 "VTBlend_Linear" 0.0 false)
    (Utilities|FlowControl|Delay 2.1)
    (bind _returnvalue_2 (UserInterface|CreateWidget "/Game/UI/W_PlayerInventory.W_PlayerInventory_C" 0 0))
    (UserInterface|Viewport|AddtoViewport _returnvalue_2 0)
    (Input|SetInputModeUIOnly _returnvalue 0 "DoNotLock")
    (Variables|/Script/Engine.PlayerController|SetbShowMouseCursor _returnvalue true)))

(event Input|ActionEvents|InputActionDash
  (params (Key :type Key%20Structure :default "None"))
  (bind _charactermovement (Variables|Character|GetCharacterMovement))
  (:Pressed
    (if (Variables|Default|GetbCanDash)
      (Variables|Default|SetbCanDash false)
      (Variables|/Script/Engine.CharacterMovementComponent|SetMaxWalkSpeed _charactermovement 1.5e+03)
      (Utilities|FlowControl|Delay 0.3)
      (Variables|/Script/Engine.CharacterMovementComponent|SetMaxWalkSpeed _charactermovement 6e+02)
      (Utilities|FlowControl|Delay 2.0)
      (Variables|Default|SetbCanDash true))))

(event Input|AxisEvents|InputAxisMoveForward
  (params (AxisValue :type Float%20%28single-precision%29))
  (Pawn|Input|AddMovementInput (Math|Vector|GetForwardVector "0, 0, 0") AxisValue false)
  (if (or (!= AxisValue 0.0) (!= (stale Input|AxisEvents|InputAxisMoveRight AxisValue) 0.0))
    (Default|CallInterruptCast)))

(event Input|AxisEvents|InputAxisMoveRight
  (params (AxisValue :type Float%20%28single-precision%29))
  (Pawn|Input|AddMovementInput (Math|Vector|GetRightVector "0, 0, 0") AxisValue false)
  (if (or (!= (stale Input|AxisEvents|InputAxisMoveForward AxisValue) 0.0) (!= AxisValue 0.0))
    (Default|CallInterruptCast)))

(fn ConstructionScript)

(fn SpendMoney
  (params (Decrease%20Money :type Integer))
  (bind _output_get (Variables|Default|SetMoney (- (Variables|Default|GetMoney) Decrease%20Money)))
  (return _output_get))