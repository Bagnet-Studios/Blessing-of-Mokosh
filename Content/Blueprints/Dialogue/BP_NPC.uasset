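; Dialogue NPC that plays line-by-line conversations from DT_Dialogues, filtered by NPC, conversation and line IDs, in a W_Dialogue widget.
; Interact advances lines while locking player shooting, rotation and movement; wife NPCs also auto-start on first overlap and cough periodically.
; When lines run out, it restores control and increments the conversation.
; Role flags then trigger shopkeeper or Auka replacement, a first-weapon chest, or campfire level travel.
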(event OnComponentEndOverlap(Box)
  (params (OverlappedComponent :type Primitive%20Component%20Object%20Reference) (OtherActor :type Actor%20Object%20Reference) (OtherComp :type Primitive%20Component%20Object%20Reference) (OtherBodyIndex :type Integer))
  (Utilities|IsValid (Variables|Default|GetDialogueWidgetRef)
    (:Is%20Valid
      (Utilities|Casting|CastToBP_PlayerCharacter OtherActor)
      (Widget|RemovefromParent (Variables|Default|GetDialogueWidgetRef))
      (Variables|Default|SetDialogueWidgetRef 0))))

(event OnComponentBeginOverlap(Box)
  (params (OverlappedComponent :type Primitive%20Component%20Object%20Reference) (OtherActor :type Actor%20Object%20Reference) (OtherComp :type Primitive%20Component%20Object%20Reference) (OtherBodyIndex :type Integer) (bFromSweep :type Boolean) (SweepResult :type Hit%20Result%20Structure%20%28by%20ref%29))
  (Utilities|FlowControl|DoOnce false
    (:Completed
      (if (Variables|Default|GetIsWife)
        (Utilities|Time|SetTimerbyEvent (delegate Custom|Cough) 4.0 true)
        (Variables|/Script/HAGJ.BaseCharacter|SetbCanShoot (Variables|Default|GetPlayerRef) false)
        (Variables|/Game/Blueprints/Player/BP_PlayerCharacter.BP_PlayerCharacter_C|SetbCanRotate (Variables|Default|GetPlayerRef) false)
        (Math|Integer|IncrementInt (Variables|Default|GetLineCurrent)
          (:%20%20
            (CallFunction|DialogueCreate)
            (if (or (Variables|Default|GetIsShop) (Variables|Default|GetIsCampFire))
              _
              (else
                (Transformation|SetActorRotation (Math|Rotator|MakeRotator 0.0 0.0 (- (.yaw (Math|Rotator|FindLookatRotation (Transformation|GetActorLocation) (Transformation|GetActorLocation (Game|GetPlayerCharacter 0)))) 6e+01)))))
            (if (not (== (Variables|Default|GetLineCurrent) 0))
              (bind _asbp_player_character (Utilities|Casting|CastToBP_PlayerCharacter (Game|GetPlayerCharacter 0)))
              (Pawn|Components|CharacterMovement|DisableMovement (Variables|/Script/Engine.Character|GetCharacterMovement _asbp_player_character)))))))))

(event Custom|Cough
  (Audio|PlaySoundatLocation "/Game/Assets/Sound/SFX/cough.cough" (Transformation|GetActorLocation) "0, 0, 0" 1.0 1.0 0.0 0 0 0))

(event EventBeginPlay
  (bind _outrownames (DataTable|GetDataTableRowNames "/Game/Blueprints/Dialogue/Data/DT_Dialogues.DT_Dialogues"))
  (for _array_element _outrownames
    (bind _returnvalue (Utilities|GetDataTableRow "/Game/Blueprints/Dialogue/Data/DT_Dialogues.DT_Dialogues" _array_element)
      (:then
        (if (== (.NPC_ID (Utilities|Struct|BreakDS_Dialogue _returnvalue)) (Variables|Default|GetNPC_ID))
          (Utilities|Array|Add (Variables|Default|GetMyDialogue) _array_element)
          (bind _asbp_player_character (Utilities|Casting|CastToBP_PlayerCharacter (Game|GetPlayerCharacter 0)))
          (Variables|Default|SetPlayerRef _asbp_player_character))))))

(event EventInteract
  (bind _returnvalue (Transformation|GetActorLocation))
  (if (Variables|Default|GetIsCampFire)
    (Effects|SpawnEmitteratLocation "/Game/Assets/FX/P_Fireside.P_Fireside" _returnvalue)
    (Audio|PlaySoundatLocation "/Game/Assets/Sound/SFX/Bonfire_01.Bonfire_01" _returnvalue "0, 0, 0" 0.3 1.0 0.0 0 0 0))
  (Variables|/Script/HAGJ.BaseCharacter|SetbCanShoot (Variables|Default|GetPlayerRef) false)
  (Variables|/Game/Blueprints/Player/BP_PlayerCharacter.BP_PlayerCharacter_C|SetbCanRotate (Variables|Default|GetPlayerRef) false)
  (Math|Integer|IncrementInt (Variables|Default|GetLineCurrent)
    (:%20%20
      (CallFunction|DialogueCreate)
      (if (or (Variables|Default|GetIsShop) (Variables|Default|GetIsCampFire))
        _
        (else
          (Transformation|SetActorRotation (Math|Rotator|MakeRotator 0.0 0.0 (- (.yaw (Math|Rotator|FindLookatRotation (Transformation|GetActorLocation) (Transformation|GetActorLocation (Game|GetPlayerCharacter 0)))) 6e+01)))))
      (if (not (== (Variables|Default|GetLineCurrent) 0))
        (bind _asbp_player_character (Utilities|Casting|CastToBP_PlayerCharacter (Game|GetPlayerCharacter 0)))
        (Pawn|Components|CharacterMovement|DisableMovement (Variables|/Script/Engine.Character|GetCharacterMovement _asbp_player_character))))))

(fn ConstructionScript)

(fn DialogueCreate
  (Utilities|IsValid (Variables|Default|GetDialogueWidgetRef)
    (:Is%20Valid
      (bind (_returned_line _returned_name) (CallFunction|DialogueGetLine))
      (Variables|/Game/UI/W_Dialogue.W_Dialogue_C|SetDialogueText (Variables|Default|GetDialogueWidgetRef) _returned_line)
      (Variables|/Game/UI/W_Dialogue.W_Dialogue_C|SetName (Variables|Default|GetDialogueWidgetRef) _returned_name))
    (:Is%20Not%20Valid
      (bind _returnvalue (UserInterface|CreateWidget "/Game/UI/W_Dialogue.W_Dialogue_C" (Game|GetPlayerController 0)))
      (bind _output_get (Variables|Default|SetDialogueWidgetRef _returnvalue))
      (UserInterface|Viewport|AddtoViewport _output_get 0)
      (bind (_returned_line_2 _returned_name_2) (CallFunction|DialogueGetLine))
      (Variables|/Game/UI/W_Dialogue.W_Dialogue_C|SetDialogueText (Variables|Default|GetDialogueWidgetRef) _returned_line_2)
      (Variables|/Game/UI/W_Dialogue.W_Dialogue_C|SetName (Variables|Default|GetDialogueWidgetRef) _returned_name_2))))

(fn DialogueGetLine
  (bind _returnvalue (Game|GetPlayerCharacter 0))
  (bind _returnvalue_2 (Transformation|GetActorTransform))
  (bind _returnvalue_3 (Transformation|GetActorTransform))
  (bind _returnvalue_4 (Transformation|GetActorTransform))
  (bind _playerref (Variables|Default|GetPlayerRef))
  (bind (_location _rotation _scale) (Math|Transform|BreakTransform _returnvalue_2))
  (bind (_location_2 _rotation_2 _scale_2) (Math|Transform|BreakTransform _returnvalue_4))
  (bind (_location_3 _rotation_3 _scale_3) (Math|Transform|BreakTransform _returnvalue_3))
  (bind _asbp_player_character (Utilities|Casting|CastToBP_PlayerCharacter _returnvalue))
  (bind _cameracomponent (Variables|/Script/HAGJ.BaseCharacter|GetCameraComponent _asbp_player_character))
  (bind _returnvalue_5 (Transformation|GetWorldRotation _cameracomponent))
  (for _array_element (Variables|Default|GetMyDialogue)
    (bind _returnvalue_6 (Utilities|GetDataTableRow "/Game/Blueprints/Dialogue/Data/DT_Dialogues.DT_Dialogues" _array_element)
      (:then
        (if (and (== (.Conversation_ID (Utilities|Struct|BreakDS_Dialogue _returnvalue_6)) (Variables|Default|GetConversation_ID)) (== (.Line_ID (Utilities|Struct|BreakDS_Dialogue _returnvalue_6)) (Variables|Default|GetLineCurrent)))
          (Utilities|Array|Add (LocalVariables|GetReturnedLines) (.Dialogue (Utilities|Struct|BreakDS_Dialogue _returnvalue_6)))
          (Utilities|Array|Add (LocalVariables|GetReturnedName) (.Name (Utilities|Struct|BreakDS_Dialogue _returnvalue_6)))))))
  (if (== (Utilities|Array|Length (LocalVariables|GetReturnedLines)) 1)
    (return (Utilities|Array|Get(acopy) (LocalVariables|GetReturnedLines)) (Utilities|Array|Get(acopy) (LocalVariables|GetReturnedName)))
    (else
      (Rendering|SetVisibility (Variables|Default|GetTextRender) false false)
      (Variables|/Game/Blueprints/Player/BP_PlayerCharacter.BP_PlayerCharacter_C|SetbCanRotate _playerref true)
      (Variables|/Script/HAGJ.BaseCharacter|SetbCanShoot _playerref true)
      (Widget|RemovefromParent (Variables|Default|GetDialogueWidgetRef))
      (Variables|Default|SetDialogueWidgetRef 0)
      (Variables|Default|SetLineCurrent 0)
      (bind _asbp_player_character_2 (Utilities|Casting|CastToBP_PlayerCharacter (Game|GetPlayerCharacter 0)))
      (Pawn|Components|CharacterMovement|SetMovementMode (Variables|/Script/Engine.Character|GetCharacterMovement _asbp_player_character_2) "MOVE_Walking" 0)
      (bind _result (Math|Integer|IncrementInt (Variables|Default|GetConversation_ID))
        (:%20%20
          (Variables|Default|SetConversation_ID _result)
          (if (Variables|Default|GetIsShop)
            (Game|SpawnActorfromClass "/Game/Blueprints/Shop/BP_Shopkeeper.BP_Shopkeeper_C" (Math|Transform|MakeTransform (Math|Vector|MakeVector (.x _location_2) (.y _location_2) (- (.z _location_2) (Variables|/Script/Engine.CapsuleComponent|GetCapsuleHalfHeight (Variables|Collision|GetCapsuleComponent)))) _rotation_2 _scale_2) "AdjustIfPossibleButAlwaysSpawn" 0 0)
            (Actor|DestroyActor)
            (elif (Variables|Default|GetIsAuka)
              (Game|SpawnActorfromClass "/Game/Blueprints/Enemy/AUKA/BP_Auka_New.BP_Auka_New_C" (Math|Transform|MakeTransform (Math|Vector|MakeVector (.x _location) (.y _location) (.z _location)) _rotation _scale) "AdjustIfPossibleButAlwaysSpawn" 0 0)
              (Actor|DestroyActor)
              (elif (Variables|Default|GetIsBatya)
                (if (not (Variables|Default|GetIsGotFirstWeapon))
                  (Game|SpawnActorfromClass "/Game/Blueprints/Environment/Chests/BP_BaseWeaponChest.BP_BaseWeaponChest_C" (Math|Transform|MakeTransform (Math|Vector|MakeVector (.x _location_3) (+ (.y _location_3) 3e+02) (- (.z _location_3) (Variables|/Script/Engine.CapsuleComponent|GetCapsuleHalfHeight (Variables|Collision|GetCapsuleComponent)))) (Math|Rotator|MakeRotator (.roll _returnvalue_5) (+ (.pitch _returnvalue_5) 4e+01) (.yaw _returnvalue_5)) _scale_3) "AdjustIfPossibleButAlwaysSpawn" 0 "/Game/Blueprints/Weapons/BP_BaseWeapon.BP_BaseWeapon_C" "You've recieved a basic sword" false 0)
                  (Variables|Default|SetIsGotFirstWeapon true))
                (elif (Variables|Default|GetIsCampFire)
                  (Game|OpenLevel(byObjectReference) "/Game/Maps/M_Level05.M_Level05"))))))))))