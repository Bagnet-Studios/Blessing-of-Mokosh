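; BP_SignPost is a signpost actor that shows its text in a dialogue widget when interacted with.
; The Interact event toggles the display, creating a W_Dialogue widget filled with MyText or removing the one already open.
; When a BP_PlayerCharacter leaves the Box component, any open widget is removed and its reference cleared.
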(event OnComponentEndOverlap(Box)
  (params (OverlappedComponent :type Primitive%20Component%20Object%20Reference) (OtherActor :type Actor%20Object%20Reference) (OtherComp :type Primitive%20Component%20Object%20Reference) (OtherBodyIndex :type Integer))
  (Utilities|IsValid (Variables|Default|GetDialogueWidgetRef)
    (:Is%20Valid
      (Utilities|Casting|CastToBP_PlayerCharacter OtherActor)
      (Widget|RemovefromParent (Variables|Default|GetDialogueWidgetRef))
      (Variables|Default|SetDialogueWidgetRef 0))))

(event EventInteract
  (Utilities|IsValid (Variables|Default|GetDialogueWidgetRef)
    (:Is%20Valid
      (Widget|RemovefromParent (Variables|Default|GetDialogueWidgetRef))
      (Variables|Default|SetDialogueWidgetRef 0))
    (:Is%20Not%20Valid
      (bind _returnvalue (UserInterface|CreateWidget "/Game/UI/W_Dialogue.W_Dialogue_C" (Game|GetPlayerController 0)))
      (bind _output_get (Variables|Default|SetDialogueWidgetRef _returnvalue))
      (UserInterface|Viewport|AddtoViewport _output_get 0)
      (Variables|/Game/UI/W_Dialogue.W_Dialogue_C|SetDialogueText (Variables|Default|GetDialogueWidgetRef) (Variables|Default|GetMyText)))))

(fn ConstructionScript)