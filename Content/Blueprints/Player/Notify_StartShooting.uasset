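; Animation notify that starts shooting for the player character by enabling attacks on its WeaponComponent.
; When received, it sets the component's ranged weapon class to BP_RangedWeapon, spawns that weapon and sets CanAttack.
; It targets player 0's BP_PlayerCharacter rather than the owner of the animated mesh.
; A separate StartMakingDamage function only sets CanAttack and is not called by the notify.
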(fn StartMakingDamage
  (bind _asbp_player_character (Utilities|Casting|CastToBP_PlayerCharacter (Game|GetPlayerCharacter 0)))
  (Variables|/Script/HAGJ.WeaponComponent|SetbCanAttack (Variables|/Script/HAGJ.BaseCharacter|GetWeaponComponent _asbp_player_character) true))

(fn ReceivedNotify
  (params (MeshComp :type Skeletal%20Mesh%20Component%20Object%20Reference) (Animation :type Anim%20Sequence%20Base%20Object%20Reference))
  (bind _asbp_player_character (Utilities|Casting|CastToBP_PlayerCharacter (Game|GetPlayerCharacter 0)))
  (Variables|/Script/HAGJ.WeaponComponent|SetRangedWeaponClass (Variables|/Script/HAGJ.BaseCharacter|GetWeaponComponent _asbp_player_character) "/Game/Blueprints/BP_RangedWeapon.BP_RangedWeapon_C")
  (Class|WeaponComponent|SpawnRangedWeapon (Variables|/Script/HAGJ.BaseCharacter|GetWeaponComponent _asbp_player_character))
  (Variables|/Script/HAGJ.WeaponComponent|SetbCanAttack (Variables|/Script/HAGJ.BaseCharacter|GetWeaponComponent _asbp_player_character) true)
  (return false))