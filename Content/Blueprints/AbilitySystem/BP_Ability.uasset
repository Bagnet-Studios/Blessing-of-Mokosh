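; Base ability actor that manages the casting phase of an ability, with an empty ActivateEffect hook.
; On BeginPlay it snaps to the caster's right-hand socket, caches player, controller and HUD references, then begins casting.
; Timed casts show a HUD cast bar and bind to its success event, while instant casts call CastAbility directly.
; CastAbility detaches the actor and calls CastSuccess, while InterruptCast destroys it and calls CastInterrupted.
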(event EventBeginPlay
  (Transformation|AttachComponentToComponent (Variables|/Script/Engine.Character|GetMesh (Variables|Default|GetCaster)) "RightHandSocket" "SnapToTarget" "SnapToTarget" "SnapToTarget" true)
  (bind _asbp_player_character (Utilities|Casting|CastToBP_PlayerCharacter (Game|GetPlayerCharacter 0)))
  (Variables|Default|SetPlayerRef _asbp_player_character)
  (bind _asbp_base_game_mode (Utilities|Casting|CastToBP_BaseGameMode (Game|GetGameMode)))
  (Variables|Default|SetHUD_UI (Variables|/Game/Blueprints/GameModes/BP_BaseGameMode.BP_BaseGameMode_C|GetHUD _asbp_base_game_mode))
  (bind _asbp_player_controller (Utilities|Casting|CastToBP_PlayerController (Game|GetPlayerController 0)))
  (Variables|Default|SetPlayer%20Controller _asbp_player_controller)
  (CallFunction|BeginCasting))

(fn ConstructionScript)

(fn BeginCasting
  (if (> (.casttime (Variables|Default|GetAbilityDetails)) 0.0)
    (bind _castbarref (Default|DisplayCastBar (Variables|Default|GetHUD_UI) self))
    (EventDispatchers|BindEventtoCastSuccesfull _castbarref (EventDispatchers|CreateEvent :!event CastAbility))
    (else
      (CallFunction|CastAbility))))

(fn CastAbility
  (Transformation|DetachFromActor "KeepWorld" "KeepWorld" "KeepWorld")
  (Default|CallCastSuccess))

(fn InterruptCast
  (Actor|DestroyActor)
  (Default|CallCastInterrupted))

(fn ActivateEffect)