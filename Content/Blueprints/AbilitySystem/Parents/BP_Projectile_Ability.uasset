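; Parent Blueprint for projectile abilities, extending a base ability with fireball cast animation and homing movement.
; On BeginPlay it starts the cast montage and, given a valid current target, sets the homing component and turns the player's yaw toward it.
; CastAbility plays the montage's EndCast section, whose notify calls ActivateEffect to launch the projectile movement and starts a stored burning sound.
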(event EventActivateEffect
  (|CallParentFunction)
  (Components|Activation|Activate (Variables|Default|GetProjectileMovement) false))

(event EventCastAbility
  (|CallParentFunction)
  (Animation|Montage|PlayMontage (Variables|/Script/Engine.Character|GetMesh (Variables|Default|GetPlayerRef)) "/Game/Blueprints/Player/Animation/AM_CastFireball.AM_CastFireball" 1.0 0.0 "EndCast"
    (:OnNotifyBegin
      (CallFunction|ActivateEffect)
      (bind _returnvalue (Audio|SpawnSound2D "/Game/Assets/Sound/SFX/Burning.Burning" 1.0 1.0 0.0 0))
      (Variables|Default|SetBurningSound _returnvalue))))

(event EventBeginPlay
  (bind _playerref (Variables|Default|GetPlayerRef))
  (bind _returnvalue (Transformation|GetActorRotation _playerref))
  (|CallParentFunction)
  (Animation|Montage|PlayMontage (Variables|/Script/Engine.Character|GetMesh (Variables|Default|GetPlayerRef)) "/Game/Blueprints/Player/Animation/AM_CastFireball.AM_CastFireball"
    (:then
      (bind _currenttarget (Variables|/Game/Blueprints/PlayerOLD/BP_PlayerController.BP_PlayerController_C|GetCurrentTarget (Variables|Default|GetPlayer%20Controller))
        (:then
          (Variables|/Script/Engine.ProjectileMovementComponent|SetHomingTargetComponent (Variables|Default|GetProjectileMovement) (Variables|/Script/Engine.Character|GetCapsuleComponent _currenttarget))
          (Transformation|SetActorRotation _playerref (Math|Rotator|MakeRotator (.roll _returnvalue) (.pitch _returnvalue) (.yaw (Math|Rotator|FindLookatRotation (Transformation|GetActorLocation (Variables|Default|GetPlayerRef)) (Transformation|GetActorLocation (Variables|/Game/Blueprints/PlayerOLD/BP_PlayerController.BP_PlayerController_C|GetCurrentTarget (Variables|Default|GetPlayer%20Controller))))))))
        (:else)))))

(fn ConstructionScript
  (|CallParentFunction))