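; BP_HolyGround_AoE is an area-of-effect ability that heals players and damages enemies standing inside it.
; On activation it sets its lifespan and starts a looping tick timer.
; Each tick, player characters overlapping the ability root gain health directly on their HealthComponent, clamped to MaxHealth, while overlapping enemy characters receive damage through ApplyDamage.
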(event Custom|TickEffect
  (Utilities|FlowControl|Sequence
    (:then_0
      (for _array_element (Collision|GetOverlappingActors (Variables|Default|GetAbilityRoot) "/Game/Blueprints/Player/BP_PlayerCharacter.BP_PlayerCharacter_C" :!class /Script/Engine.PrimitiveComponent)
        (bind _asbp_player_character (Utilities|Casting|CastToBP_PlayerCharacter _array_element))
        (Variables|/Script/HAGJ.HealthComponent|SetHealth (Variables|/Script/HAGJ.BaseCharacter|GetHealthComponent _asbp_player_character) (Math|Float|Clamp(Float) (+ (Variables|/Script/HAGJ.HealthComponent|GetHealth (Variables|/Script/HAGJ.BaseCharacter|GetHealthComponent _asbp_player_character)) (Variables|Default|GetHealPerDot)) 0.0 (Variables|/Script/HAGJ.HealthComponent|GetMaxHealth (Variables|/Script/HAGJ.BaseCharacter|GetHealthComponent _asbp_player_character))))))
    (:then_1
      (for _array_element_2 (Collision|GetOverlappingActors (Variables|Default|GetAbilityRoot) "/Game/Blueprints/Enemy/BP_EnemyCharacter.BP_EnemyCharacter_C" :!class /Script/Engine.PrimitiveComponent)
        (Game|Damage|ApplyDamage _array_element_2 (Variables|Default|GetDamagePerDot) 0 0)))))

(event EventActivateEffect
  (|CallParentFunction)
  (Actor|SetLifeSpan (Variables|Default|GetLifeSpan))
  (Utilities|Time|SetTimerbyEvent (delegate Custom|TickEffect) (Variables|Default|GetDotTimer) true))

(fn ConstructionScript
  (|CallParentFunction))