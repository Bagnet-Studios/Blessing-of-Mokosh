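; Fortitude buff actor that doubles the player's weapon damage for as long as it exists.
; On BeginPlay it gets player 0's BP_PlayerCharacter and sets DamageMultiplier to double on the WeaponComponent's current weapon and current projectile.
; EndPlay sets both multipliers back to a fixed 1.0 rather than their prior values, acting on whatever weapon and projectile are current at that moment.
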(event EventBeginPlay
  (|CallParentFunction)
  (bind _asbp_player_character (Utilities|Casting|CastToBP_PlayerCharacter (Game|GetPlayerCharacter 0)))
  (bind _weaponcomponent (Variables|/Script/HAGJ.BaseCharacter|GetWeaponComponent _asbp_player_character)
    (:then
      (bind _currentweapon (Variables|/Script/HAGJ.WeaponComponent|GetCurrentWeapon _weaponcomponent)
        (:then
          (Variables|/Script/HAGJ.BaseWeapon|SetDamageMultiplier _currentweapon 2.0)
          (bind _currentprojectile (Variables|/Script/HAGJ.WeaponComponent|GetCurrentProjectile _weaponcomponent)
            (:then
              (Variables|/Script/HAGJ.BaseProjectile|SetDamageMultiplier _currentprojectile 2.0))
            (:else)))
        (:else)))
    (:else)))

(event EventEndPlay
  (params (EndPlayReason :type EEndPlayReason%20Enum :default "Destroyed"))
  (bind _asbp_player_character (Utilities|Casting|CastToBP_PlayerCharacter (Game|GetPlayerCharacter 0)))
  (bind _weaponcomponent (Variables|/Script/HAGJ.BaseCharacter|GetWeaponComponent _asbp_player_character)
    (:then
      (bind _currentweapon (Variables|/Script/HAGJ.WeaponComponent|GetCurrentWeapon _weaponcomponent)
        (:then
          (Variables|/Script/HAGJ.BaseWeapon|SetDamageMultiplier _currentweapon 1.0)
          (bind _currentprojectile (Variables|/Script/HAGJ.WeaponComponent|GetCurrentProjectile _weaponcomponent)
            (:then
              (Variables|/Script/HAGJ.BaseProjectile|SetDamageMultiplier _currentprojectile 1.0))
            (:else)))
        (:else)))
    (:else)))

(fn ConstructionScript
  (|CallParentFunction))