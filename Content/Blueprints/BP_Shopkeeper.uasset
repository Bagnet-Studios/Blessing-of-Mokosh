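; BP_Shopkeeper is an interactable shop NPC that switches the player into a shop screen.
; Interact plays a talk sound, hides the current weapon, and disables movement and input.
; If the ShopTrigger overlap's OtherActor is the player, it blends the camera to itself, shows the cursor and hides the character.
; After a short delay, it opens W_Shopkeeper with a self-reference and re-enables input in UI-only mode.
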(event OnComponentBeginOverlap(ShopTrigger)
  (params (OverlappedComponent :type Primitive%20Component%20Object%20Reference) (OtherActor :type Actor%20Object%20Reference) (OtherComp :type Primitive%20Component%20Object%20Reference) (OtherBodyIndex :type Integer) (bFromSweep :type Boolean) (SweepResult :type Hit%20Result%20Structure%20%28by%20ref%29)))

(event EventInteract
  (bind _returnvalue (Game|GetPlayerController 0))
  (Audio|PlaySoundatLocation "/Game/Assets/Sound/SFX/AITalk.AITalk" (Transformation|GetActorLocation) "0, 0, 0" 1.0 1.0 0.0 0 0 0)
  (bind _asbp_player_character (Utilities|Casting|CastToBP_PlayerCharacter (Game|GetPlayerCharacter 0)))
  (Rendering|SetActorHiddenInGame (Variables|/Script/HAGJ.WeaponComponent|GetCurrentWeapon (Variables|/Script/HAGJ.BaseCharacter|GetWeaponComponent _asbp_player_character)) true)
  (Pawn|Components|CharacterMovement|DisableMovement (Variables|/Script/Engine.Character|GetCharacterMovement (.AsBP%20Player%20Character (Utilities|Casting|CastToBP_PlayerCharacter (Game|GetPlayerCharacter 0)))))
  (Input|DisableInput (Game|GetPlayerController 0) 0)
  (if (== (stale OnComponentBeginOverlap(ShopTrigger) OtherActor) (Game|GetPlayerCharacter 0))
    (Game|Player|SetViewTargetwithBlend (Game|GetPlayerController 0) self 1.0 "VTBlend_Linear" 0.0 false)
    (Input|SetInputModeUIOnly _returnvalue 0 "DoNotLock")
    (Variables|/Script/Engine.PlayerController|SetbShowMouseCursor _returnvalue true)
    (Rendering|SetActorHiddenInGame (Game|GetPlayerCharacter 0) true)
    (Utilities|FlowControl|Delay 1.1)
    (bind _returnvalue_2 (UserInterface|CreateWidget "/Game/UI/W_Shopkeeper.W_Shopkeeper_C" 0 self))
    (UserInterface|Viewport|AddtoViewport _returnvalue_2 0)
    (Input|EnableInput (Game|GetPlayerController 0) 0)))

(fn ConstructionScript)