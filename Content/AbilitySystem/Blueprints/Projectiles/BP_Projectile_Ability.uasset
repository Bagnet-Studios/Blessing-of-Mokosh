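; Projectile ability Blueprint that ties a fireball cast animation on the player to the launch of its projectile.
; On BeginPlay it plays the fireball montage on the player's mesh, and CastAbility replays it from the EndCast section.
; A montage notify during that section calls ActivateEffect, which activates projectile movement, syncing the launch to the animation.
; Each event also runs its parent implementation.
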(event EventActivateEffect
  (|CallParentFunction)
  (Components|Activation|Activate (Variables|Default|GetProjectileMovement) false))

(event EventCastAbility
  (|CallParentFunction)
  (Animation|Montage|PlayMontage (Variables|/Script/Engine.Character|GetMesh (Variables|Default|GetPlayerRef)) "/Game/AbilitySystem/Animations/AM_Fireball.AM_Fireball" 1.0 0.0 "EndCast"
    (:OnNotifyBegin
      (CallFunction|ActivateEffect))))

(event EventBeginPlay
  (|CallParentFunction)
  (Animation|Montage|PlayMontage (Variables|/Script/Engine.Character|GetMesh (Variables|Default|GetPlayerRef)) "/Game/AbilitySystem/Animations/AM_Fireball.AM_Fireball"))

(fn ConstructionScript
  (|CallParentFunction))