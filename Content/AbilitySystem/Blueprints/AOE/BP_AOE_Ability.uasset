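; Area-of-effect ability actor that plays a standing AoE cast montage on the player and spawns its Niagara effect on the ground beneath them.
; CastAbility runs the parent logic and plays the montage, whose notify begin triggers ActivateEffect.
; ActivateEffect runs the parent logic, activates Niagara, zeroes the actor's rotation and moves it to the hit point of a downward trace from the player character.
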(event EventActivateEffect
  (bind _returnvalue (Game|GetPlayerCharacter 0))
  (bind _returnvalue_2 (Transformation|GetActorLocation _returnvalue))
  (|CallParentFunction)
  (Components|Activation|Activate (Variables|Default|GetNiagara) false)
  (Transformation|SetActorRotation "0, 0, 0")
  (bind _outhit (Collision|LineTraceByChannel _returnvalue_2 (+ _returnvalue_2 "0,0,-10000.000000") "TraceTypeQuery1" false (Utilities|Array|MakeArray _returnvalue) "None"))
  (Transformation|SetActorLocation (.location _outhit) false false))

(event EventCastAbility
  (|CallParentFunction)
  (Animation|Montage|PlayMontage (Variables|/Script/Engine.Character|GetMesh (Variables|Default|GetPlayerRef)) "/Game/AbilitySystem/Animations/AM_StandingAoE.AM_StandingAoE"
    (:OnNotifyBegin
      (CallFunction|ActivateEffect))))

(fn ConstructionScript
  (|CallParentFunction))