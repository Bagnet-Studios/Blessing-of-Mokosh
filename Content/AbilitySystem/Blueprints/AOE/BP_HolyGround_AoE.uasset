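; BP_HolyGround_AoE is a timed area-of-effect ability, named as holy ground, that periodically affects player characters standing inside it.
; On activation it runs the parent logic, sets its lifespan and starts a looping timer at the DotTimer interval.
; Each tick passes HealPerDot through ApplyDamage to every BP_PlayerCharacter overlapping AbilityRoot, so healing uses the damage pipeline.
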(event Custom|TickEffect
  (for _array_element (Collision|GetOverlappingActors (Variables|Default|GetAbilityRoot) "/Game/Blueprints/BP_PlayerCharacter.BP_PlayerCharacter_C" :!class /Script/Engine.PrimitiveComponent)
    (Game|Damage|ApplyDamage _array_element (Variables|Default|GetHealPerDot) 0 0)))

(event EventActivateEffect
  (|CallParentFunction)
  (Actor|SetLifeSpan (Variables|Default|GetLifeSpan))
  (Utilities|Time|SetTimerbyEvent (delegate Custom|TickEffect) (Variables|Default|GetDotTimer) true))

(fn ConstructionScript
  (|CallParentFunction))