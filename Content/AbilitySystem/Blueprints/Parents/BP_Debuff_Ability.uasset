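; BP_Debuff_Ability is a parent ability actor for debuffs placed on the player controller's current target, playing a standing AoE montage on the player at BeginPlay.
; On cast it destroys itself if the target already carries the same class, sets its lifespan, attaches to the target and refreshes the target UI.
; A looping timer calls DebuffTick, which is empty here.
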(event Custom|DebuffTick)

(event EventBeginPlay
  (|CallParentFunction)
  (Animation|Montage|PlayMontage (Variables|/Script/Engine.Character|GetMesh (Variables|Default|GetPlayerRef)) "/Game/AbilitySystem/Animations/AM_StandingAoE.AM_StandingAoE"))

(event EventCastAbility
  (|CallParentFunction)
  (CallFunction|ClearDuplicates)
  (Actor|SetLifeSpan (Variables|Default|GetDebuffLifespan))
  (CallFunction|ApplyDebuff)
  (bind _returnvalue (Utilities|Time|SetTimerbyEvent (delegate Custom|DebuffTick) (Variables|Default|GetDebuffTickrate) true))
  (Variables|Default|SetDebuffTickTimer _returnvalue))

(fn ConstructionScript
  (|CallParentFunction))

(fn ClearDuplicates
  (bind _self self)
  (for _array_element (Actor|GetAttachedActors (Variables|/Game/Blueprints/BP_PlayerController.BP_PlayerController_C|GetCurrentTarget (Variables|Default|GetPlayer%20Controller)) true)
    (if (and (== (Utilities|GetClass _array_element) (Utilities|GetClass _self)) (!= _array_element _self))
      (Actor|DestroyActor))))

(fn ApplyDebuff
  (bind _asbp_player_controller (Utilities|Casting|CastToBP_PlayerController (Game|GetPlayerController 0)))
  (Transformation|AttachActorToActor (Variables|/Game/Blueprints/BP_PlayerController.BP_PlayerController_C|GetCurrentTarget _asbp_player_controller) "None" "SnapToTarget" "SnapToTarget" "SnapToTarget" true)
  (Default|UpdateTargetUI (Variables|/Game/AbilitySystem/UI/W_HUD.W_HUD_C|GetW_TargetUI (Variables|Default|GetHUD_UI))))