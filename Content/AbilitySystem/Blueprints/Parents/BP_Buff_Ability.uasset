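; Parent Blueprint for buff abilities, providing a timed lifespan, periodic tick and HUD buff panel entry.
; BeginPlay destroys same-class actors attached to the caster, then plays a casting montage on the player.
; CastAbility spawns a spark effect, sets the lifespan, adds the buff to the UI and starts a looping tick timer.
; TickBuff and ClearBuff are empty stubs, and EndPlay calls CallBuffRemoved.
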(event Custom|TickBuff)

(event EventBeginPlay
  (CallFunction|ClearDuplicates)
  (|CallParentFunction)
  (Animation|Montage|PlayMontage (Variables|/Script/Engine.Character|GetMesh (Variables|Default|GetPlayerRef)) "/Game/AbilitySystem/Animations/AM_StandingAoE.AM_StandingAoE"))

(event EventCastAbility
  (Niagara|SpawnSystematLocation "/Game/FX/N_Spark_System.N_Spark_System" (Transformation|GetActorLocation))
  (Actor|SetLifeSpan (Variables|Default|GetBuffLifeSpan))
  (CallFunction|ApplyBuff)
  (bind _returnvalue (Utilities|Time|SetTimerbyEvent (delegate Custom|TickBuff) (Variables|Default|GetBuffTickrate) true))
  (Variables|Default|SetBuffTickTimer _returnvalue))

(event EventEndPlay
  (params (EndPlayReason :type EEndPlayReason%20Enum :default "Destroyed"))
  (Default|CallBuffRemoved))

(fn ConstructionScript
  (|CallParentFunction))

(fn ApplyBuff
  (Default|AddBufftoUI (Variables|/Game/AbilitySystem/UI/W_HUD.W_HUD_C|GetW_BuffPanel (Variables|Default|GetHUD_UI)) self))

(fn ClearBuff)

(fn ClearDuplicates
  (for _array_element (Actor|GetAttachedActors (Variables|Default|GetCaster) true)
    (if (== (Utilities|GetClass _array_element) (Utilities|GetClass self))
      (Actor|DestroyActor _array_element))))